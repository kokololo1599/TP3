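; BP_SDTAIController is an AI controller that runs its behavior tree under time-slicing rather than per-frame ticking.
; On BeginPlay it starts the behavior tree, disables the brain component's tick and registers itself with the AI time slicer subsystem, presumably leaving tree updates to that subsystem.
; On EndPlay it unregisters from the subsystem.
; The move-completed handler is an empty stub whose binding never runs.
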(event `self.ReceiveBeginPlay`
  (`self.RunBehaviorTree` "/Game/Blueprint/AIBehaviorTree.AIBehaviorTree")
  (`ActorComponent.SetComponentTickEnabled` (`self.BrainComponent`) false)
  (`AITimeSlicerSubsystem.RegisterController` (subsystem `AITimeSlicerSubsystem`) self))

(event `self.ReceiveEndPlay`
  (params (EndPlayReason :type "EEndPlayReason Enum" :default "Destroyed"))
  (`AITimeSlicerSubsystem.UnregisterController` (subsystem `AITimeSlicerSubsystem`) self))

(event `ReceiveMoveCompleted_Event` :!signature `self.ReceiveMoveCompleted`
  (params (RequestID :type "AIRequestID Structure") (Result :type "EPathFollowingResult Enum" :default "Success")))

(fn `UserConstructionScript`)